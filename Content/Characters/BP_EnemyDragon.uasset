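; BP_EnemyDragon is a dragon enemy character that chases the player and attacks at close range.
; On BeginPlay it assigns itself as owner of its widget health bar, then starts a looping AI MoveTo toward the player pawn.
; Each successful move calls OnAttack and waits briefly before moving again, while a failed move retries immediately.
; The OnDeadImplement event hides the health bar widget.
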(event EventBeginPlay
  (Utilities|FlowControl|Sequence
    (:then_0
      (bind _asui_hpbar (Utilities|Casting|CastToUI_HPBar (UserInterface|GetWidget (Variables|Default|GetWidget))))
      (Variables|/Game/UI/UI_HPBar.UI_HPBar_C|SetOwner _asui_hpbar self))
    (:then_1
      (AI|AIMoveTo self "0, 0, 0" (Game|Player|GetPlayerPawn 0) 8e+01 false :!label _label
        (:OnSuccess
          (Class|PaperCharacterEnemyBase|OnAttack)
          (Utilities|FlowControl|Delay 1.0)
          (goto _label))
        (:OnFail
          (goto _label))))))

(event EventOnDeadImplement
  (Development|SetHiddeninGame (Variables|Default|GetWidget) true false))

(fn ConstructionScript)