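; BP_EnemyJinn is an enemy character that binds its HP bar widget to itself and hides it on death.
; On BeginPlay it loops an AI move to a random navigable point within a short radius, keeping only the X so it moves along one axis.
; Each successful move triggers an attack and a short delay before the next, while a failed move retries at once.
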(event EventBeginPlay
  (bind _returnvalue (Transformation|GetActorLocation))
  (bind (_x _y _z) (Math|Vector|BreakVector _returnvalue))
  (Utilities|FlowControl|Sequence
    (:then_0
      (bind _asui_hpbar (Utilities|Casting|CastToUI_HPBar (UserInterface|GetWidget (Variables|Default|GetWidget))))
      (Variables|/Game/UI/UI_HPBar.UI_HPBar_C|SetOwner _asui_hpbar self))
    (:then_1
      (AI|AIMoveTo self (Math|Vector|MakeVector (.X (Math|Vector|BreakVector (.RandomLocation (Class|NavigationSystemV1|GetRandomPointinNavigableRadius _returnvalue 1.5e+02 0 0)))) _y _z) 0 1.0 false :!label _label
        (:OnSuccess
          (Class|PaperCharacterEnemyBase|OnAttack)
          (Utilities|FlowControl|Delay 2.0)
          (goto _label))
        (:OnFail
          (goto _label))))))

(event EventOnDeadImplement
  (Development|SetHiddeninGame (Variables|Default|GetWidget) true false))

(fn ConstructionScript)